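; Key pickup actor for the medieval dungeon, collected with the Interact action while the player is near it.
; A box overlap toggles input on the key, while actor overlap shows and removes a press-E prompt widget.
; Interacting finds the KeyInventory_BP widget on screen, increments its KeysCollected count, destroys the key and plays a 2D piano sound.
; The key count lives directly in the inventory widget.
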(event OnComponentBeginOverlap(Box)
  (params (OverlappedComponent :type Primitive%20Component%20Object%20Reference) (OtherActor :type Actor%20Object%20Reference) (OtherComp :type Primitive%20Component%20Object%20Reference) (OtherBodyIndex :type Integer) (bFromSweep :type Boolean) (SweepResult :type Hit%20Result%20Structure%20%28by%20ref%29))
  ;[1 1 1] Player Controller Input on Box Collision
  (Input|EnableInput (Game|GetPlayerController 0)))

(event OnComponentEndOverlap(Box)
  (params (OverlappedComponent :type Primitive%20Component%20Object%20Reference) (OtherActor :type Actor%20Object%20Reference) (OtherComp :type Primitive%20Component%20Object%20Reference) (OtherBodyIndex :type Integer))
  ;[1 1 1] Player Controller Input on Box Collision
  (Input|DisableInput (Game|GetPlayerController 0)))

(event Collision|EventActorEndOverlap
  (params (OtherActor :type Actor%20Object%20Reference))
  ;[1 1 1] Add/Remove Press E Inter Widget
  (Widget|RemovefromParent (Variables|Default|GetPress%20ERef)))

(event Collision|EventActorBeginOverlap
  (params (OtherActor :type Actor%20Object%20Reference))
  ;[1 1 1] Add/Remove Press E Inter Widget
  (bind _returnvalue (UserInterface|CreateWidget "/Game/StarterContent/Widgets/PressEInterface.PressEInterface_C"))
  (UserInterface|Viewport|AddtoViewport _returnvalue 0)
  (Variables|Default|SetPress%20ERef _returnvalue))

(event EventTick
  (params (DeltaSeconds :type Float%20%28single-precision%29)))

(event EventBeginPlay)

(event Input|ActionEvents|InputActionInteract
  (params (Key :type Key%20Structure :default "None"))
  ;[1 1 1] Add/Destroy Key
  (:Pressed
    (bind _foundwidgets (Widget|GetAllWidgetsOfClass "/Game/StarterContent/Widgets/KeyInventory_BP.KeyInventory_BP_C" true))
    (bind _askey_inventory_bp (Utilities|Casting|CastToKeyInventory_BP (Utilities|Array|Get(acopy) _foundwidgets)))
    (Variables|/Game/StarterContent/Widgets/KeyInventory_BP.KeyInventory_BP_C|SetKeysCollected _askey_inventory_bp (+ (Variables|/Game/StarterContent/Widgets/KeyInventory_BP.KeyInventory_BP_C|GetKeysCollected _askey_inventory_bp) 1.0))
    (Actor|DestroyActor)
    (Audio|SpawnSound2D "/Game/Sounds/Horror_Game_Sounds/Cues/Piano_NO_ECHO_Cue.Piano_NO_ECHO_Cue" 0.5 1.0 0.0 0)))

(fn ConstructionScript)