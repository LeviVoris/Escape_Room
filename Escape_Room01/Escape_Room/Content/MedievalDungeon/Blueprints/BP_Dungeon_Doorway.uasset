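; BP_Dungeon_Doorway is an interactive dungeon double door that the player opens and closes with E.
; Left and right box overlaps enable or disable input, while actor overlap adds or removes a Press E prompt widget.
; E plays or reverses one timeline per leaf to drive its yaw.
; Tick writes both timeline values to one shared ClosedDoor flag, so only the left door's value sticks.
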(event OnComponentBeginOverlap(RBox)
  (params (OverlappedComponent :type Primitive%20Component%20Object%20Reference) (OtherActor :type Actor%20Object%20Reference) (OtherComp :type Primitive%20Component%20Object%20Reference) (OtherBodyIndex :type Integer) (bFromSweep :type Boolean) (SweepResult :type Hit%20Result%20Structure%20%28by%20ref%29))
  ;[1 1 1] Player Controller Input Control
  (Input|EnableInput (Game|GetPlayerController 0)))

(event OnComponentEndOverlap(RBox)
  (params (OverlappedComponent :type Primitive%20Component%20Object%20Reference) (OtherActor :type Actor%20Object%20Reference) (OtherComp :type Primitive%20Component%20Object%20Reference) (OtherBodyIndex :type Integer))
  ;[1 1 1] Player Controller Input Control
  (Input|DisableInput (Game|GetPlayerController 0)))

(event OnComponentBeginOverlap(LBox)
  (params (OverlappedComponent :type Primitive%20Component%20Object%20Reference) (OtherActor :type Actor%20Object%20Reference) (OtherComp :type Primitive%20Component%20Object%20Reference) (OtherBodyIndex :type Integer) (bFromSweep :type Boolean) (SweepResult :type Hit%20Result%20Structure%20%28by%20ref%29))
  ;[1 1 1] Player Controller Input Control
  (Input|EnableInput (Game|GetPlayerController 0)))

(event OnComponentEndOverlap(LBox)
  (params (OverlappedComponent :type Primitive%20Component%20Object%20Reference) (OtherActor :type Actor%20Object%20Reference) (OtherComp :type Primitive%20Component%20Object%20Reference) (OtherBodyIndex :type Integer))
  ;[1 1 1] Player Controller Input Control
  (Input|DisableInput (Game|GetPlayerController 0)))

(event Collision|EventActorEndOverlap
  (params (OtherActor :type Actor%20Object%20Reference))
  ;[1 1 1] Add/Remove Press E Inter Widget
  (Widget|RemovefromParent (Variables|Default|GetPress%20E%20Ref)))

(event Collision|EventActorBeginOverlap
  (params (OtherActor :type Actor%20Object%20Reference))
  ;[1 1 1] Add/Remove Press E Inter Widget
  (bind _returnvalue (UserInterface|CreateWidget "/Game/MedievalDungeon/Blueprints/PressEInterface.PressEInterface_C"))
  (UserInterface|Viewport|AddtoViewport _returnvalue 0)
  (Variables|Default|SetPress%20E%20Ref _returnvalue))

(event EventTick
  (params (DeltaSeconds :type Float%20%28single-precision%29))
  ;[1 1 1] E Input Command
  (Variables|Default|SetClosedDoor (< (stale Input|KeyboardEvents|E _dooropen) 1.0))
  (Variables|Default|SetClosedDoor (< (stale Input|KeyboardEvents|E _dooropen) 1.0)))

(event EventBeginPlay)

(event Input|KeyboardEvents|E
  (params (Key :type Key%20Structure :default "None"))
  ;[1 1 1] E Input Command
  (:Pressed
    (if (Variables|Default|GetClosedDoor)
      (bind _dooropen (Timeline|Timeline_0 Play)
        (:Update
          (Transformation|SetRelativeRotation (Variables|Default|GetSM_DoorWay_Large_Door_Right) (Math|Rotator|MakeRotator 0.0 0.0 _dooropen) false false)))
      (else
        (Timeline|Timeline_0 Reverse)))))

(event Input|KeyboardEvents|E
  (params (Key :type Key%20Structure :default "None"))
  ;[1 1 1] E Input Command
  (:Pressed
    (if (Variables|Default|GetClosedDoor)
      (bind _dooropen (Timeline|Timeline_1 Play)
        (:Update
          (Transformation|SetRelativeRotation (Variables|Default|GetSM_DoorWay_Large_Door_Left) (Math|Rotator|MakeRotator 0.0 0.0 _dooropen) false false)))
      (else
        (Timeline|Timeline_1 Reverse)))))

(fn ConstructionScript)